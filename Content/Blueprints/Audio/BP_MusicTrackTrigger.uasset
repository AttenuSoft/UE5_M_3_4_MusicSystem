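; BP_MusicTrackTrigger is a placeable trigger volume that controls music when a BP_Character overlaps its region.
; On overlap it calls the character's music player component to either start a named track with the assigned music data, stop that track, or stop all tracks.
; The construction script labels the trigger with the track name and a color-coded Play, Clear or ClearAll tag for readability in the level.
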(event `self.ReceiveBeginPlay`
  (add `PrimitiveComponent.OnComponentBeginOverlap` (`self.TriggerRegion`) (delegate `OnTriggerRegionBeginOverlap`)))

(event `OnTriggerRegionBeginOverlap`
  (params (OverlappedComponent :type "PrimitiveComponent Object Reference") (OtherActor :type "Actor Object Reference") (OtherComp :type "PrimitiveComponent Object Reference") (OtherBodyIndex :type Integer) (bFromSweep :type Boolean) (SweepResult :type "HitResult Structure (by ref)"))
  (bind _asbp_character (cast `/Game/Blueprints/Character/BP_Character` OtherActor))
  (if (`self.bClearTrack`)
    (if (`self.bClearAllTracks`)
      (bind _bp_musicplayercomponent (`/Game/Blueprints/Character/BP_Character.BP_MusicPlayerComponent` _asbp_character))
      (`MusicPlayerComponent.StopAllMusicTracks` _bp_musicplayercomponent)
      (else
        (`MusicPlayerComponent.StopSpecificMusicTrack` _bp_musicplayercomponent (`self.TrackName`))))
    (else
      (set `MusicPlayerComponent.CurrentMusicData` (`self.MusicData`) (`/Game/Blueprints/Character/BP_Character.BP_MusicPlayerComponent` _asbp_character))
      (`MusicPlayerComponent.CreateNewMusicTrack` _bp_musicplayercomponent (`self.TrackName`)))))

(fn `UserConstructionScript`
  (bind _shouldclear_text (`self.ShouldClear_Text`))
  (`TextRenderComponent.K2_SetText` (`self.TrackName_Text`) (`KismetTextLibrary.Conv_NameToText` (`self.TrackName`)))
  (`TextRenderComponent.K2_SetText` _shouldclear_text (`KismetMathLibrary.SelectText` (`KismetMathLibrary.SelectText` "(ClearAll)" "(Clear)" (`self.bClearAllTracks`)) "(Play)" (`self.bClearTrack`)))
  (`TextRenderComponent.SetTextRenderColor` _shouldclear_text (select `bool` (`self.bClearTrack`) :`false` (`KismetMathLibrary.LinearColor_ToRGBE` (struct :`R` 0.127211 :`G` 1.0 :`A` 1.0)) :`true` (`KismetMathLibrary.LinearColor_ToRGBE` (struct :`R` 1.0 :`G` 0.002106 :`A` 1.0)))))