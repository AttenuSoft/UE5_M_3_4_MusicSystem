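; Single music track audio component that prints on-screen debug messages when its track starts and stops.
; On BeginPlay it binds to its started and stopped delegates, and each handler unbinds itself on first firing, so each reports only once.
; A shared print event shows track name and next track, plus primary sound duration on start, color-coded and keyed per track and state.
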(event `self.ReceiveBeginPlay`
  (add `self.OnSingleMusicTrackStarted` (delegate `OnTrackStarted`))
  (add `self.OnSingleMusicTrackStopped` (delegate `OnTrackStopped`)))

(event `OnTrackStarted`
  (remove `self.OnSingleMusicTrackStarted` (delegate `OnTrackStarted`))
  (`self.PrintTrackData` true))

(event `OnTrackStopped`
  (remove `self.OnSingleMusicTrackStopped` (delegate `OnTrackStopped`))
  (`self.PrintTrackData` false))

(event `PrintTrackData`
  (params (bOnTrackStarted :type Boolean))
  (bind _nexttrack (`self.NextTrack`))
  (bind _trackname (`self.TrackName`))
  (bind _sound (`AudioComponent.Sound` (`self.PrimaryAudioComponent`)))
  (if bOnTrackStarted
    (`KismetSystemLibrary.PrintText` (`|FormatText` "NEW SINGLE TRACK STARTED \nSingle track name:           {a} \nSingle track duration:      {b} \nNext track:                         {c}" _trackname (select `bool` (`KismetSystemLibrary.IsValid` _sound) :`true` (`SoundBase.Duration` _sound)) _nexttrack) true true (struct :`R` 0.156485 :`G` 1.0 :`A` 1.0) 10.0 (`KismetStringLibrary.Conv_StringToName` (`KismetStringLibrary.Concat_StrStr` (`KismetStringLibrary.Conv_NameToString` (`self.TrackName`)) "started")))
    (else
      (`KismetSystemLibrary.PrintText` (`|FormatText` "SINGLE TRACK STOPPED \nSingle track name:           {a} \nNext track:                         {b}" _trackname _nexttrack) true true (struct :`R` 1.0 :`B` 0.041073 :`A` 1.0) 5.0 (`KismetStringLibrary.Conv_StringToName` (`KismetStringLibrary.Concat_StrStr` (`KismetStringLibrary.Conv_NameToString` (`self.TrackName`)) "stopped"))))))