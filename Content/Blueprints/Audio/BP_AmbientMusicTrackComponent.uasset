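; Audio component that schedules layered ambient music, made of a pad plus primary and secondary decorator tracks, on a Quartz clock.
; SetupQuartzClock creates and starts the decorator clock at a given BPM, subscribed to all quantization events.
; Each change of beat number calls PlayTrack, then prints debug info on music frequency, per-layer countdowns, current tracks and the valid pad and decorator pools.
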(event `self.ReceiveBeginPlay`
  (set `self.CurrentMusicFrequency` 9))

(event `self.SetupQuartzClock`
  (params (BeatsPerMinute :type "Float (single-precision)"))
  (bind _returnvalue (`QuartzSubsystem.CreateNewClock` (subsystem `QuartzSubsystem`) (`self.DecoratorClock`) (`self.DecoratorClockSettings`) false true))
  (bind _output_get (set `self.DecoratorClockHandle` _returnvalue))
  (bind _clockhandle (`QuartzClockHandle.SetBeatsPerMinute` :`self` _output_get :`BeatsPerMinute` BeatsPerMinute))
  (bind _clockhandle_2 (`QuartzClockHandle.SubscribeToAllQuantizationEvents` _clockhandle (`|CreateDelegate` :!event `OnQuartzClockBeat`)))
  (`QuartzClockHandle.StartClock` _clockhandle_2))

(event `OnQuartzClockBeat`
  (params (ClockName :type Name) (QuantizationType :type "EQuartzCommandQuantization Enum" :default "Bar") (NumBars :type Integer) (Beat :type Integer) (BeatFraction :type "Float (single-precision)"))
  (bind _beatsbeforenexttrack (`self.BeatsBeforeNextTrack`))
  (bind _padcomponent (`self.PadComponent`))
  (bind _primarydecoratorcomponent (`self.PrimaryDecoratorComponent`))
  (bind _secondarydecoratorcomponent (`self.SecondaryDecoratorComponent`))
  (if (!= (`self.CurrentBeat`) Beat)
    (set `self.CurrentBeat` Beat)
    (`|ExecutionSequence`
      (:`then_0`
        (`self.PlayTrack`))
      (:`then_1`
        (`KismetSystemLibrary.PrintText` (`|FormatText` "Current music frequency: {a} \n" (`self.CurrentMusicFrequency`)) true false (struct :`R` 1.0 :`G` 0.463483 :`A` 1.0) 2.0 "Frequency")
        (`KismetSystemLibrary.PrintText` (`|FormatText` "Beats before next track: \n          Pad:                {a} \n          Primary:        {b} \n          Secondary:   {c} \n \nCurrent ambient tracks: \n          Pad:                {d} \n          Primary:        {e} \n          Secondary:   {f} " (`|GetArrayItem` _beatsbeforenexttrack) (`|GetArrayItem` _beatsbeforenexttrack 1) (`|GetArrayItem` _beatsbeforenexttrack 2) (select `bool` (`KismetSystemLibrary.IsValid` _padcomponent) :`false` "*Waiting*" :`true` (`DecoratorComponent.DecoratorName` _padcomponent)) (select `bool` (`KismetSystemLibrary.IsValid` _primarydecoratorcomponent) :`false` "*Waiting*" :`true` (`DecoratorComponent.DecoratorName` _primarydecoratorcomponent)) (select `bool` (`KismetSystemLibrary.IsValid` _secondarydecoratorcomponent) :`false` "*Waiting*" :`true` (`DecoratorComponent.DecoratorName` _secondarydecoratorcomponent))) true false (struct :`R` 1.0 :`B` 0.075234 :`A` 1.0) 2.0 "AmbientDecoratorTrackInfo")
        (`KismetSystemLibrary.PrintText` "Valid pads:" true false (struct :`G` 1.0 :`B` 0.107649 :`A` 1.0) 2.0 "Pads")
        (for _array_element (`self.ValidPads`)
          (`KismetSystemLibrary.PrintText` (`|FormatText` "Pad name: {a}" (break `AmbientPad` _array_element)) true false (struct :`R` 0.00543 :`G` 1.0 :`A` 1.0) 2.0 (break `AmbientPad` _array_element)))
        (`KismetSystemLibrary.PrintText` " \nValid decorators:" true false (struct :`G` 0.66 :`B` 1.0 :`A` 1.0) 2.0 "Decorators")
        (for _array_element_2 (`self.ValidDecorators`)
          (`KismetSystemLibrary.PrintText` (`|FormatText` "Decorator name: {a}     Decorators remaining: {b}" (break `AmbientDecoratorWrapper` _array_element_2) (`KismetArrayLibrary.Array_Length` (`.Decorator` (break `AmbientDecoratorWrapper` _array_element_2)))) true false (struct :`G` 0.66 :`B` 1.0 :`A` 1.0) 2.0 (break `AmbientDecoratorWrapper` _array_element_2)))))))