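; Player controller that sets up Enhanced Input and drives movement, camera look and running for the player character.
; BeginPlay adds the IMC_Move mapping context, whose input actions act on player character 0 rather than a cached pawn reference.
; Move actions add input along the control rotation's forward and right vectors, while Turn and LookUp add yaw and pitch.
; Run raises max walk speed while triggered and lowers it on completion.
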(event `self.ReceiveBeginPlay`
  (`EnhancedInputSubsystemInterface.AddMappingContext` (subsystem `EnhancedInputLocalPlayerSubsystem`) "/Game/Blueprints/Character/EnhancedInput/Context/IMC_Move.IMC_Move" 0 (struct)))

(event `EnhancedInput|/Game/Blueprints/Character/EnhancedInput/InputAction/IA_MoveFoward`
  (params (ActionValue :type "Float (double-precision)") (ElapsedSeconds :type "Float (double-precision)") (TriggeredSeconds :type "Float (double-precision)") (InputAction :type "InputAction Object Reference" :default "/Game/Blueprints/Character/EnhancedInput/InputAction/IA_MoveFoward.IA_MoveFoward"))
  (bind _returnvalue (`GameplayStatics.GetPlayerCharacter` 0))
  (:`Triggered`
    (`Pawn.AddMovementInput` _returnvalue (`KismetMathLibrary.GetForwardVector` (`Pawn.GetControlRotation` _returnvalue)) ActionValue false)))

(event `EnhancedInput|/Game/Blueprints/Character/EnhancedInput/InputAction/IA_MoveRight`
  (params (ActionValue :type "Float (double-precision)") (ElapsedSeconds :type "Float (double-precision)") (TriggeredSeconds :type "Float (double-precision)") (InputAction :type "InputAction Object Reference" :default "/Game/Blueprints/Character/EnhancedInput/InputAction/IA_MoveRight.IA_MoveRight"))
  (bind _returnvalue (`GameplayStatics.GetPlayerCharacter` 0))
  (:`Triggered`
    (`Pawn.AddMovementInput` _returnvalue (`KismetMathLibrary.GetRightVector` (`Pawn.GetControlRotation` _returnvalue)) ActionValue false)))

(event `EnhancedInput|/Game/Blueprints/Character/EnhancedInput/InputAction/IA_Turn`
  (params (ActionValue :type "Float (double-precision)") (ElapsedSeconds :type "Float (double-precision)") (TriggeredSeconds :type "Float (double-precision)") (InputAction :type "InputAction Object Reference" :default "/Game/Blueprints/Character/EnhancedInput/InputAction/IA_Turn.IA_Turn"))
  (:`Triggered`
    (`Pawn.AddControllerYawInput` (`GameplayStatics.GetPlayerCharacter` 0) ActionValue)))

(event `EnhancedInput|/Game/Blueprints/Character/EnhancedInput/InputAction/IA_LookUp`
  (params (ActionValue :type "Float (double-precision)") (ElapsedSeconds :type "Float (double-precision)") (TriggeredSeconds :type "Float (double-precision)") (InputAction :type "InputAction Object Reference" :default "/Game/Blueprints/Character/EnhancedInput/InputAction/IA_LookUp.IA_LookUp"))
  (:`Triggered`
    (`Pawn.AddControllerPitchInput` (`GameplayStatics.GetPlayerCharacter` 0) ActionValue)))

(event `EnhancedInput|/Game/Blueprints/Character/EnhancedInput/InputAction/IA_Run`
  (params (ActionValue :type Boolean) (ElapsedSeconds :type "Float (double-precision)") (TriggeredSeconds :type "Float (double-precision)") (InputAction :type "InputAction Object Reference" :default "/Game/Blueprints/Character/EnhancedInput/InputAction/IA_Run.IA_Run"))
  (bind _charactermovement (`Character.CharacterMovement` (`GameplayStatics.GetPlayerCharacter` 0)))
  (:`Triggered`
    (set `CharacterMovementComponent.MaxWalkSpeed` 1000.0 _charactermovement))
  (:`Completed`
    (set `CharacterMovementComponent.MaxWalkSpeed` 600.0 _charactermovement)))

(fn `UserConstructionScript`)