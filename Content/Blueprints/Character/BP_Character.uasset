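; BP_Character is a character Blueprint that owns the frequency slider UI widget.
; On BeginPlay it creates WBP_FrequencySlider, stores it as SliderWidget, and adds it to the viewport hidden and disabled.
; Two custom events enable or disable the slider by toggling its visibility and enabled state after a validity check, reusing the same widget instance.
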(event `self.ReceiveBeginPlay`
  (bind _returnvalue (`|CreateWidget` "/Game/Blueprints/Widgets/WBP_FrequencySlider.WBP_FrequencySlider_C"))
  (bind _output_get (set `self.SliderWidget` _returnvalue))
  (`Widget.SetVisibility` _output_get "Hidden")
  (`Widget.SetIsEnabled` _output_get false)
  (`UserWidget.AddToViewport` _output_get 0))

(event `EnableFrequencySliderWidget`
  (bind _sliderwidget (`self.SliderWidget`)
    (:`then`
      (`Widget.SetVisibility` _sliderwidget "Visible")
      (`Widget.SetIsEnabled` _sliderwidget true))
    (:`else`)))

(event `DisableFrequencySliderWidget`
  (bind _sliderwidget (`self.SliderWidget`)
    (:`then`
      (`Widget.SetVisibility` _sliderwidget "Hidden")
      (`Widget.SetIsEnabled` _sliderwidget false))
    (:`else`)))

(fn `UserConstructionScript`)